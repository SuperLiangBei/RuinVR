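; VR hand actor that binds itself to a VRCharacter's left or right motion controller, chosen by its VRHand setting.
; On BeginPlay it stays tickable during pause and runs RegisterAndSetOwningPawn.
; Without a supplied pawn, it casts its owner, stores itself on that character, snap-attaches to the controller and calls RegisterHands.
; A valid supplied pawn only refreshes the pawn and controller references and enables tick.
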(event EventBeginPlay
  ;[1 1 1] BeginPlay
  (Utilities|FlowControl|Sequence
    (:then_0
      (Class|Actor|SetTickablewhenPaused true) ; 当暂停时当前对象正常运动
    )
    (:then_1
      (CallFunction|RegisterandSetOwningPawn))))

(event Collision|EventActorBeginOverlap
  (params (OtherActor :type Actor%20Object%20Reference)))

(event EventTick
  (params (DeltaSeconds :type Float%20%28single-precision%29)))

(fn ConstructionScript)

(fn RegisterandSetOwningPawn
  (params (UpdatePawn :type VR%20Character%20Object%20Reference))
  (bind _self self)
  (Utilities|IsValid UpdatePawn
    (:Is%20Valid
      ;[1 1 1] 如果有新的Pawn的情况
      (Variables|Pawn|SetVRPawn UpdatePawn)
      (Actor|Tick|SetActorTickEnabled true)
      (Utilities|HandSwitch (Variables|Pawn|GetVRHand)
        (:Left
          (Variables|Default|SetVRMotionController (Variables|/Game/Blueprints/Game/VRCharacter.VRCharacter_C|GetVRMotionController_Left (Variables|Pawn|GetVRPawn))))
        (:Right
          (Variables|Default|SetVRMotionController (Variables|/Game/Blueprints/Game/VRCharacter.VRCharacter_C|GetVRMotionController_Right (Variables|Pawn|GetVRPawn)))))
      (return))
    (:Is%20Not%20Valid
      ;[1 1 1] 尚未有Owning的Pawn的情况，把Hand绑定到Pawn中的运动控制器上，并区别左手和右手
      (bind _asvrcharacter (Utilities|Casting|CastToVRCharacter (Components|GetOwner)))
      (Variables|Pawn|SetVRPawn _asvrcharacter)
      (Actor|Tick|SetActorTickEnabled true)
      (Utilities|HandSwitch (Variables|Pawn|GetVRHand)
        (:Left
          (Variables|/Game/Blueprints/Game/VRCharacter.VRCharacter_C|SetLeftHandBP (Variables|Pawn|GetVRPawn) _self)
          (bind _output_get (Variables|Default|SetVRMotionController (Variables|/Game/Blueprints/Game/VRCharacter.VRCharacter_C|GetVRMotionController_Left (Variables|Pawn|GetVRPawn))))
          (Transformation|AttachComponentToComponent _output_get "None" "SnapToTarget" "SnapToTarget" "KeepWorld" false))
        (:Right
          (Variables|/Game/Blueprints/Game/VRCharacter.VRCharacter_C|SetRightHandBP (Variables|Pawn|GetVRPawn) _self)
          (bind _output_get_2 (Variables|Default|SetVRMotionController (Variables|/Game/Blueprints/Game/VRCharacter.VRCharacter_C|GetVRMotionController_Right (Variables|Pawn|GetVRPawn))))
          (Transformation|AttachComponentToComponent _output_get_2 "None" "SnapToTarget" "SnapToTarget" "KeepWorld" false)))
      (Default|RegisterHands (Variables|Pawn|GetVRPawn))
      (return))))